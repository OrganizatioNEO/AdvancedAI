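; BP_BlankTile is a scenario generation tile that starts undecided and settles into one of eight straight, corner or double-corner layouts.
; Tick counts the remaining entries in Possibilities, but the auto-solve on a single possibility is disconnected.
; PickRandom chooses a remaining option and calls SetState, which locks the tile and shows its pieces.
; Four edge getters derive each side's connection from piece visibility, in a style resembling wave function collapse.
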(event Custom|PickRandom
  (bind _possiblesolutions (Variables|Default|GetPossibleSolutions))
  (if (not (Variables|Default|GetSolved))
    (Utilities|Array|Clear (Variables|Default|GetPossibleSolutions))
    (for (_array_element _array_index) (Variables|Default|GetPossibilities)
      (if _array_element
        (Utilities|Array|Add _possiblesolutions _array_index)))
    (CallFunction|SetState (Utilities|Array|Get(acopy) _possiblesolutions (Math|Random|RandomInteger (Utilities|Array|Length _possiblesolutions))))))

(event Custom|SetState
  (params (Tile :type Integer))
  (if (not (Variables|Default|GetSolved))
    (Variables|Default|SetSolution Tile)
    (Variables|Default|SetSolved true)
    (switch int Tile
      (:0
        (Rendering|SetVisibility (Variables|Default|GetNS) true false))
      (:1
        (Rendering|SetVisibility (Variables|Default|GetEW) true false))
      (:2
        (Rendering|SetVisibility (Variables|Default|GetNE) true false :!label _label))
      (:3
        (Rendering|SetVisibility (Variables|Default|GetSE) true false :!label _label_2))
      (:4
        (Rendering|SetVisibility (Variables|Default|GetSW) true false :!label _label_3))
      (:5
        (Rendering|SetVisibility (Variables|Default|GetNW) true false :!label _label_4))
      (:6
        (Utilities|FlowControl|Sequence
          (:then_0
            (goto _label))
          (:then_1
            (goto _label_3))))
      (:7
        (Utilities|FlowControl|Sequence
          (:then_0
            (goto _label_2))
          (:then_1
            (goto _label_4)))))))

(event EventBeginPlay)

(event Collision|EventActorBeginOverlap
  (params (OtherActor :type Actor%20Object%20Reference)))

(event EventTick
  (params (DeltaSeconds :type Float%20%28single-precision%29))
  (if (not (Variables|Default|GetSolved))
    (Variables|Default|SetAmountTrue 0)
    (for (_array_element _array_index) (Variables|Default|GetPossibilities)
      (if _array_element
        (Math|Integer|IncrementInt (Variables|Default|GetAmountTrue)
          (:%20%20
            (Variables|Default|SetSolution _array_index)))))))

(fn ConstructionScript)

(fn GetNorthEdge
  (return (or (or (Rendering|IsVisible (Variables|Default|GetNW)) (Rendering|IsVisible (Variables|Default|GetNE))) (Rendering|IsVisible (Variables|Default|GetNS)))))

(fn GetEastEdge
  (return (or (or (Rendering|IsVisible (Variables|Default|GetSE)) (Rendering|IsVisible (Variables|Default|GetNE))) (Rendering|IsVisible (Variables|Default|GetEW)))))

(fn GetSouthEdge
  (return (or (or (Rendering|IsVisible (Variables|Default|GetSE)) (Rendering|IsVisible (Variables|Default|GetSW))) (Rendering|IsVisible (Variables|Default|GetNS)))))

(fn GetWestEdge
  (return (or (or (Rendering|IsVisible (Variables|Default|GetNW)) (Rendering|IsVisible (Variables|Default|GetSW))) (Rendering|IsVisible (Variables|Default|GetEW)))))