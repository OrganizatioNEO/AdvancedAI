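; Scenario-generation tile actor that tracks which tile options remain possible and displays the chosen one, in the style of a constraint solver.
; CheckSolutions adds each true entry in the Possibilities array to AmountTrue.
; Tick marks the tile solved when that count is exactly one, storing that entry's index as Solution, and unsolved when it is higher.
; SetSolution applies the dynamic material from the matching Tiles entry to the Plane.
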(event Custom|CheckSolutions
  (bind _array_element (Utilities|Array|ForEachLoopwithBreak (Variables|Default|GetPossibilities))
    (:LoopBody
      (if _array_element
        (Math|Integer|IncrementInt (Variables|Default|GetAmountTrue))))))

(event Custom|SetSolution
  (bind _returnvalue (Appearance|GetDynamicMaterial (Utilities|Array|Get(acopy) (Variables|Default|GetTiles) (Variables|Default|GetSolution)) :!class /Script/UMG.Image))
  (Rendering|Material|SetMaterial (Variables|Default|GetPlane) 0 _returnvalue))

(event EventBeginPlay)

(event Collision|EventActorBeginOverlap
  (params (OtherActor :type Actor%20Object%20Reference)))

(event EventTick
  (params (DeltaSeconds :type Float%20%28single-precision%29))
  (Math|Integer|CompareInt (Variables|Default|GetAmountTrue) 1
    (:>
      (Variables|Default|SetSolved false))
    (:==
      (Variables|Default|SetSolved true)
      (bind (_array_element _array_index) (Utilities|Array|ForEachLoopwithBreak (Variables|Default|GetPossibilities) :!label _label)
        (:LoopBody
          (if _array_element
            (Variables|Default|SetSolution _array_index)
            (goto _label Break)))))))

(fn ConstructionScript)