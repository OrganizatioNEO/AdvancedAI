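; BP_TTTBoard is a tic-tac-toe board actor that enables player input and gathers its nine compass-named cells into a Slots array.
; A left click traces from the deprojected mouse position on the Visibility channel with persistent debug drawing, then prints the hit component's name.
; SetSlot applies an O or X material according to CurrentTurnO, but the cast-and-place branch calling it is disconnected and the turn never toggles.
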(event Custom|SetSlot
  (params (Slot :type Static%20Mesh%20Component%20Object%20Reference))
  (if (Variables|Default|GetCurrentTurnO)
    (Rendering|Material|SetMaterial Slot 0 "/Game/TicTacToe/Mat_O.Mat_O")
    (else
      (Rendering|Material|SetMaterial Slot 0 "/Game/TicTacToe/Mat_X.Mat_X"))))

(event EventBeginPlay
  (Input|EnableInput (Game|GetPlayerController 0))
  (Variables|Default|SetSlots (Utilities|Array|MakeArray (Variables|Default|GetNW) (Variables|Default|GetN) (Variables|Default|GetNE) (Variables|Default|GetW) (Variables|Default|GetC) (Variables|Default|GetE) (Variables|Default|GetSW) (Variables|Default|GetS) (Variables|Default|GetSE))))

(event Collision|EventActorBeginOverlap
  (params (OtherActor :type Actor%20Object%20Reference)))

(event EventTick
  (params (DeltaSeconds :type Float%20%28single-precision%29)))

(event Input|MouseEvents|LeftMouseButton
  (params (Key :type Key%20Structure :default "None"))
  (bind _returnvalue (Game|GetPlayerController 0))
  (bind (_worldlocation _worlddirection) (Game|Player|ConvertMouseLocationToWorldSpace _returnvalue))
  (:Pressed
    (bind (_outhit _returnvalue_2) (Collision|LineTraceByChannel _worldlocation (+ _worldlocation (* _worlddirection 1e+04)) "TraceTypeQuery1" false 0 "Persistent"))
    (if _returnvalue_2
      (Development|PrintString (Utilities|GetDisplayName (.HitComponent (Collision|BreakHitResult _outhit)))))))

(fn ConstructionScript)