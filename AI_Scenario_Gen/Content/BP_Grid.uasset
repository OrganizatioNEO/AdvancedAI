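; BP_Grid procedurally fills a grid of BP_BlankTile actors with a simplified Wave Function Collapse.
; BeginPlay spawns tiles into a position-keyed map, fixes the centre tile's state and queues its neighbours.
; Each Tick either refills the frontier from solved cells or updates frontier possibilities from solved neighbours' edges, then randomly resolves the first entry.
; Lowest-entropy selection exists but is disconnected, so tiles resolve in queue order.
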(event Custom|FilterToExplore
  (for _array_element (Variables|Default|GetToExplore)
    (Utilities|FlowControl|Sequence ; check if top/bot/left/right compatible
      (:then_0
        (if (.ReturnValue (Utilities|Map|Find (Variables|Default|GetGrid) (+ _array_element "0.000000,-1.000000,0.000000")))
          (if (Utilities|Array|ContainsItem (Variables|Default|GetSolved) (+ _array_element "0.000000,-1.000000,0.000000"))
            (if (Default|GetSouthEdge (.Value (Utilities|Map|Find (Variables|Default|GetGrid) (+ _array_element "0.000000,-1.000000,0.000000"))))
              (Utilities|Array|SetArrayElem (Variables|/Game/BP_BlankTile.BP_BlankTile_C|GetPossibilities (.Value (Utilities|Map|Find (Variables|Default|GetGrid) _array_element))) 1 false)
              (Utilities|Array|SetArrayElem (Variables|/Game/BP_BlankTile.BP_BlankTile_C|GetPossibilities (.Value (Utilities|Map|Find (Variables|Default|GetGrid) _array_element))) 3 false)
              (Utilities|Array|SetArrayElem (Variables|/Game/BP_BlankTile.BP_BlankTile_C|GetPossibilities (.Value (Utilities|Map|Find (Variables|Default|GetGrid) _array_element))) 4 false)
              (else
                (Utilities|Array|SetArrayElem (Variables|/Game/BP_BlankTile.BP_BlankTile_C|GetPossibilities (.Value (Utilities|Map|Find (Variables|Default|GetGrid) _array_element))) 0 false)
                (Utilities|Array|SetArrayElem (Variables|/Game/BP_BlankTile.BP_BlankTile_C|GetPossibilities (.Value (Utilities|Map|Find (Variables|Default|GetGrid) _array_element))) 2 false)
                (Utilities|Array|SetArrayElem (Variables|/Game/BP_BlankTile.BP_BlankTile_C|GetPossibilities (.Value (Utilities|Map|Find (Variables|Default|GetGrid) _array_element))) 5 false)
                (Utilities|Array|SetArrayElem (Variables|/Game/BP_BlankTile.BP_BlankTile_C|GetPossibilities (.Value (Utilities|Map|Find (Variables|Default|GetGrid) _array_element))) 6 false)
                (Utilities|Array|SetArrayElem (Variables|/Game/BP_BlankTile.BP_BlankTile_C|GetPossibilities (.Value (Utilities|Map|Find (Variables|Default|GetGrid) _array_element))) 7 false))))))
      (:then_1
        (if (.ReturnValue (Utilities|Map|Find (Variables|Default|GetGrid) (+ _array_element "0.000000,1.000000,0.000000")))
          (if (Utilities|Array|ContainsItem (Variables|Default|GetSolved) (+ _array_element "0.000000,1.000000,0.000000"))
            (if (Default|GetNorthEdge (.Value (Utilities|Map|Find (Variables|Default|GetGrid) (+ _array_element "0.000000,1.000000,0.000000"))))
              (Utilities|Array|SetArrayElem (Variables|/Game/BP_BlankTile.BP_BlankTile_C|GetPossibilities (.Value (Utilities|Map|Find (Variables|Default|GetGrid) _array_element))) 1 false)
              (Utilities|Array|SetArrayElem (Variables|/Game/BP_BlankTile.BP_BlankTile_C|GetPossibilities (.Value (Utilities|Map|Find (Variables|Default|GetGrid) _array_element))) 2 false)
              (Utilities|Array|SetArrayElem (Variables|/Game/BP_BlankTile.BP_BlankTile_C|GetPossibilities (.Value (Utilities|Map|Find (Variables|Default|GetGrid) _array_element))) 5 false)
              (else
                (Utilities|Array|SetArrayElem (Variables|/Game/BP_BlankTile.BP_BlankTile_C|GetPossibilities (.Value (Utilities|Map|Find (Variables|Default|GetGrid) _array_element))) 0 false)
                (Utilities|Array|SetArrayElem (Variables|/Game/BP_BlankTile.BP_BlankTile_C|GetPossibilities (.Value (Utilities|Map|Find (Variables|Default|GetGrid) _array_element))) 3 false)
                (Utilities|Array|SetArrayElem (Variables|/Game/BP_BlankTile.BP_BlankTile_C|GetPossibilities (.Value (Utilities|Map|Find (Variables|Default|GetGrid) _array_element))) 4 false)
                (Utilities|Array|SetArrayElem (Variables|/Game/BP_BlankTile.BP_BlankTile_C|GetPossibilities (.Value (Utilities|Map|Find (Variables|Default|GetGrid) _array_element))) 6 false)
                (Utilities|Array|SetArrayElem (Variables|/Game/BP_BlankTile.BP_BlankTile_C|GetPossibilities (.Value (Utilities|Map|Find (Variables|Default|GetGrid) _array_element))) 7 false))))))
      (:then_2
        (if (.ReturnValue (Utilities|Map|Find (Variables|Default|GetGrid) (+ _array_element "-1.000000,0.000000,0.000000")))
          (if (Utilities|Array|ContainsItem (Variables|Default|GetSolved) (+ _array_element "-1.000000,0.000000,0.000000"))
            (if (Default|GetEastEdge (.Value (Utilities|Map|Find (Variables|Default|GetGrid) (+ _array_element "-1.000000,0.000000,0.000000"))))
              (Utilities|Array|SetArrayElem (Variables|/Game/BP_BlankTile.BP_BlankTile_C|GetPossibilities (.Value (Utilities|Map|Find (Variables|Default|GetGrid) _array_element))) 0 false)
              (Utilities|Array|SetArrayElem (Variables|/Game/BP_BlankTile.BP_BlankTile_C|GetPossibilities (.Value (Utilities|Map|Find (Variables|Default|GetGrid) _array_element))) 2 false)
              (Utilities|Array|SetArrayElem (Variables|/Game/BP_BlankTile.BP_BlankTile_C|GetPossibilities (.Value (Utilities|Map|Find (Variables|Default|GetGrid) _array_element))) 3 false)
              (else
                (Utilities|Array|SetArrayElem (Variables|/Game/BP_BlankTile.BP_BlankTile_C|GetPossibilities (.Value (Utilities|Map|Find (Variables|Default|GetGrid) _array_element))) 1 false)
                (Utilities|Array|SetArrayElem (Variables|/Game/BP_BlankTile.BP_BlankTile_C|GetPossibilities (.Value (Utilities|Map|Find (Variables|Default|GetGrid) _array_element))) 4 false)
                (Utilities|Array|SetArrayElem (Variables|/Game/BP_BlankTile.BP_BlankTile_C|GetPossibilities (.Value (Utilities|Map|Find (Variables|Default|GetGrid) _array_element))) 5 false)
                (Utilities|Array|SetArrayElem (Variables|/Game/BP_BlankTile.BP_BlankTile_C|GetPossibilities (.Value (Utilities|Map|Find (Variables|Default|GetGrid) _array_element))) 6 false)
                (Utilities|Array|SetArrayElem (Variables|/Game/BP_BlankTile.BP_BlankTile_C|GetPossibilities (.Value (Utilities|Map|Find (Variables|Default|GetGrid) _array_element))) 7 false))))))
      (:then_3
        (if (.ReturnValue (Utilities|Map|Find (Variables|Default|GetGrid) (+ _array_element "1.000000,0.000000,0.000000")))
          (if (Utilities|Array|ContainsItem (Variables|Default|GetSolved) (+ _array_element "1.000000,0.000000,0.000000"))
            (if (Default|GetWestEdge (.Value (Utilities|Map|Find (Variables|Default|GetGrid) (+ _array_element "1.000000,0.000000,0.000000"))))
              (Utilities|Array|SetArrayElem (Variables|/Game/BP_BlankTile.BP_BlankTile_C|GetPossibilities (.Value (Utilities|Map|Find (Variables|Default|GetGrid) _array_element))) 0 false)
              (Utilities|Array|SetArrayElem (Variables|/Game/BP_BlankTile.BP_BlankTile_C|GetPossibilities (.Value (Utilities|Map|Find (Variables|Default|GetGrid) _array_element))) 4 false)
              (Utilities|Array|SetArrayElem (Variables|/Game/BP_BlankTile.BP_BlankTile_C|GetPossibilities (.Value (Utilities|Map|Find (Variables|Default|GetGrid) _array_element))) 5 false)
              (else
                (Utilities|Array|SetArrayElem (Variables|/Game/BP_BlankTile.BP_BlankTile_C|GetPossibilities (.Value (Utilities|Map|Find (Variables|Default|GetGrid) _array_element))) 1 false)
                (Utilities|Array|SetArrayElem (Variables|/Game/BP_BlankTile.BP_BlankTile_C|GetPossibilities (.Value (Utilities|Map|Find (Variables|Default|GetGrid) _array_element))) 2 false)
                (Utilities|Array|SetArrayElem (Variables|/Game/BP_BlankTile.BP_BlankTile_C|GetPossibilities (.Value (Utilities|Map|Find (Variables|Default|GetGrid) _array_element))) 3 false)
                (Utilities|Array|SetArrayElem (Variables|/Game/BP_BlankTile.BP_BlankTile_C|GetPossibilities (.Value (Utilities|Map|Find (Variables|Default|GetGrid) _array_element))) 6 false)
                (Utilities|Array|SetArrayElem (Variables|/Game/BP_BlankTile.BP_BlankTile_C|GetPossibilities (.Value (Utilities|Map|Find (Variables|Default|GetGrid) _array_element))) 7 false)))))))))

(event Custom|UpdateToExplore
  (bind _solved (Variables|Default|GetSolved))
  (for (_ _array_index) _solved
    (Utilities|FlowControl|Sequence
      (:then_0
        (if (.ReturnValue (Utilities|Map|Find (Variables|Default|GetGrid) (+ (Utilities|Array|Get(acopy) _solved _array_index) "1.000000,0.000000,0.000000")))
          (if (not (Utilities|Array|ContainsItem (Variables|Default|GetToExplore) (+ (Utilities|Array|Get(acopy) _solved _array_index) "1.000000,0.000000,0.000000")))
            (if (not (Utilities|Array|ContainsItem (Variables|Default|GetSolved) (+ (Utilities|Array|Get(acopy) _solved _array_index) "1.000000,0.000000,0.000000")))
              (Utilities|Array|Add (Variables|Default|GetToExplore) (+ (Utilities|Array|Get(acopy) _solved _array_index) "1.000000,0.000000,0.000000"))))))
      (:then_1
        (if (.ReturnValue (Utilities|Map|Find (Variables|Default|GetGrid) (+ (Utilities|Array|Get(acopy) _solved _array_index) "-1.000000,0.000000,0.000000")))
          (if (not (Utilities|Array|ContainsItem (Variables|Default|GetToExplore) (+ (Utilities|Array|Get(acopy) _solved _array_index) "-1.000000,0.000000,0.000000")))
            (if (not (Utilities|Array|ContainsItem (Variables|Default|GetSolved) (+ (Utilities|Array|Get(acopy) _solved _array_index) "-1.000000,0.000000,0.000000")))
              (Utilities|Array|Add (Variables|Default|GetToExplore) (+ (Utilities|Array|Get(acopy) _solved _array_index) "-1.000000,0.000000,0.000000"))))))
      (:then_2
        (if (.ReturnValue (Utilities|Map|Find (Variables|Default|GetGrid) (+ (Utilities|Array|Get(acopy) _solved _array_index) "0.000000,1.000000,0.000000")))
          (if (not (Utilities|Array|ContainsItem (Variables|Default|GetToExplore) (+ (Utilities|Array|Get(acopy) _solved _array_index) "0.000000,1.000000,0.000000")))
            (if (not (Utilities|Array|ContainsItem (Variables|Default|GetSolved) (+ (Utilities|Array|Get(acopy) _solved _array_index) "0.000000,1.000000,0.000000")))
              (Utilities|Array|Add (Variables|Default|GetToExplore) (+ (Utilities|Array|Get(acopy) _solved _array_index) "0.000000,1.000000,0.000000"))))))
      (:then_3
        (if (.ReturnValue (Utilities|Map|Find (Variables|Default|GetGrid) (+ (Utilities|Array|Get(acopy) _solved _array_index) "0.000000,-1.000000,0.000000")))
          (if (not (Utilities|Array|ContainsItem (Variables|Default|GetToExplore) (+ (Utilities|Array|Get(acopy) _solved _array_index) "0.000000,-1.000000,0.000000")))
            (if (not (Utilities|Array|ContainsItem (Variables|Default|GetSolved) (+ (Utilities|Array|Get(acopy) _solved _array_index) "0.000000,-1.000000,0.000000")))
              (Utilities|Array|Add (Variables|Default|GetToExplore) (+ (Utilities|Array|Get(acopy) _solved _array_index) "0.000000,-1.000000,0.000000")))))))))

(event Custom|SolveFirstToExplore
  (bind _toexplore (Variables|Default|GetToExplore))
  (bind _output (Utilities|Array|Get(acopy) _toexplore))
  (Default|PickRandom (.Value (Utilities|Map|Find (Variables|Default|GetGrid) _output)))
  (Utilities|Array|Add (Variables|Default|GetSolved) _output)
  (Utilities|Array|RemoveItem _toexplore _output))

(event EventBeginPlay
  (bind _columns (Variables|Default|GetColumns))
  (bind _rows (Variables|Default|GetRows))
  (bind _returnvalue (/ _rows 2))
  (bind _returnvalue_2 (/ _columns 2))
  (bind _returnvalue_3 (Math|Conversions|ToFloat(Integer) _returnvalue))
  (bind _returnvalue_4 (Math|Conversions|ToFloat(Integer) _returnvalue_2))
  (bind _returnvalue_5 (Math|Vector|MakeVector _returnvalue_4 _returnvalue_3 1.0))
  ;[1 1 1] Spawn Initial Grid
  (for _index (range 0 (Variables|Default|GetColumns))
    (for _index_2 (range 0 (Variables|Default|GetRows))
      (bind _returnvalue_6 (Game|SpawnActorfromClass "/Game/BP_BlankTile.BP_BlankTile_C" (Math|Conversions|ToTransform(Vector) (* (Math|Vector|MakeVector (Math|Conversions|ToFloat(Integer) _index) (Math|Conversions|ToFloat(Integer) _index_2) 1.0) "100.000000,100.000000,10.000000")) "Undefined" "MultiplyWithRoot" 0 0))
      (Utilities|Map|Add (Variables|Default|GetGrid) (Math|Vector|MakeVector (Math|Conversions|ToFloat(Integer) _index) (Math|Conversions|ToFloat(Integer) _index_2) 1.0) _returnvalue_6)
      (Utilities|Array|Add (Variables|Default|GetMapKeys) (Math|Vector|MakeVector (Math|Conversions|ToFloat(Integer) _index) (Math|Conversions|ToFloat(Integer) _index_2) 1.0))))
  (bind _output_get (Variables|Default|SetOrigin _returnvalue_5))
  (Default|SetState (.Value (Utilities|Map|Find (Variables|Default|GetGrid) _returnvalue_5)) 6)
  (Utilities|Array|Add (Variables|Default|GetSolved) _output_get)
  (Utilities|FlowControl|Sequence
    (:then_0
      (if (.ReturnValue (Utilities|Map|Find (Variables|Default|GetGrid) (+ (Variables|Default|GetOrigin) "1.000000,0.000000,0.000000")))
        (Utilities|Array|Add (Variables|Default|GetToExplore) (+ (Variables|Default|GetOrigin) "1.000000,0.000000,0.000000"))))
    (:then_1
      (if (.ReturnValue (Utilities|Map|Find (Variables|Default|GetGrid) (+ (Variables|Default|GetOrigin) "-1.000000,0.000000,0.000000")))
        (Utilities|Array|Add (Variables|Default|GetToExplore) (+ (Variables|Default|GetOrigin) "-1.000000,0.000000,0.000000"))))
    (:then_2
      (if (.ReturnValue (Utilities|Map|Find (Variables|Default|GetGrid) (+ (Variables|Default|GetOrigin) "0.000000,1.000000,0.000000")))
        (Utilities|Array|Add (Variables|Default|GetToExplore) (+ (Variables|Default|GetOrigin) "0.000000,1.000000,0.000000"))))
    (:then_3
      (if (.ReturnValue (Utilities|Map|Find (Variables|Default|GetGrid) (+ (Variables|Default|GetOrigin) "0.000000,-1.000000,0.000000")))
        (Utilities|Array|Add (Variables|Default|GetToExplore) (+ (Variables|Default|GetOrigin) "0.000000,-1.000000,0.000000"))))))

(event Collision|EventActorBeginOverlap
  (params (OtherActor :type Actor%20Object%20Reference)))

(event EventTick
  (params (DeltaSeconds :type Float%20%28single-precision%29))
  (if (< (Utilities|Array|Length (Variables|Default|GetSolved)) (Utilities|Array|Length (Variables|Default|GetMapKeys)))
    (if (Utilities|Array|IsEmpty (Variables|Default|GetToExplore))
      (CallFunction|UpdatetoExplore)
      (else
        (CallFunction|FiltertoExplore)
        (CallFunction|SolveFirsttoExplore)))))

(fn ConstructionScript)